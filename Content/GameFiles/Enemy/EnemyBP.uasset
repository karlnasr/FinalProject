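; EnemyBP is an enemy that chases the player and is destroyed when its health runs out.
; On BeginPlay it casts and stores the player character, then starts ChasePlayer.
; ChasePlayer runs AI MoveTo toward the player and calls itself again on success or failure, keeping the pursuit going indefinitely.
; AnyDamage subtracts damage from clamped health and destroys the actor at zero.
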(event Custom|Chase%20Player
  (params (PlayerToChase :type Ue%204ASP%20Character%20Object%20Reference))
  (AI|AIMoveTo self "0, 0, 0" PlayerToChase 5.0 false
    (:OnSuccess
      _)
    (:OnFail
      _))
  (CallFunction|ChasePlayer (Variables|Default|GetChar%20REF)))

(event EventBeginPlay
  (bind _asue_4asp_character (Utilities|Casting|CastToUe4ASP_Character (Game|GetPlayerCharacter 0)))
  (bind _output_get (Variables|Default|SetChar%20REF _asue_4asp_character))
  (CallFunction|ChasePlayer _output_get))

(event Game|Damage|EventAnyDamage
  (params (Damage :type Float%20%28single-precision%29) (DamageType :type Damage%20Type%20Object%20Reference) (InstigatedBy :type Controller%20Object%20Reference) (DamageCauser :type Actor%20Object%20Reference))
  (bind _output_get (Variables|Default|SetHealth (Math|Float|Clamp(Float) (- (Variables|Default|GetHealth) Damage) 0.0 1e+02)))
  (if (== _output_get 0.0)
    (Actor|DestroyActor)))

(fn ConstructionScript)